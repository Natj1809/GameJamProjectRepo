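; BP_SpawnMaster runs an enemy wave, spawning BP_ChasingEnemy at random spawn points and printing a win message once all are dead.
; The construction script gathers every BP_SpawnLocation and sets itself as each one's Master.
; BeginPlay asks randomly picked locations, repeats allowed, to spawn a fixed batch, incrementing a Spawned counter.
; The EnemyDeath event decrements that counter and declares victory when it reaches zero.
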(event Custom|EnemyDeath
  (bind _result (Math|Integer|DecrementInt (Variables|Default|GetSpawned))
    (:%20%20
      (if (<= _result 0)
        (Development|PrintString "We WON")))))

(event EventBeginPlay
  (for _index (range 0 5)
    (Default|Spawn (Utilities|Array|Get(acopy) (Variables|Default|GetLocations) (Math|Random|RandomIntegerinRange 0 (- (Utilities|Array|Length (Variables|Default|GetLocations)) 1))) "/Game/OurContent/EnemyCopy/ChaseEnemy/BP_ChasingEnemy.BP_ChasingEnemy_C")
    (Math|Integer|IncrementInt (Variables|Default|GetSpawned))))

(fn ConstructionScript
  (bind _outactors (Actor|GetAllActorsOfClass "/Game/OurContent/SpawningCopy/BP_SpawnLocation.BP_SpawnLocation_C"))
  (bind _output_get (Variables|Default|SetLocations _outactors))
  (for _array_element _output_get
    (Variables|/Game/OurContent/SpawningCopy/BP_SpawnLocation.BP_SpawnLocation_C|SetMaster _array_element self)))