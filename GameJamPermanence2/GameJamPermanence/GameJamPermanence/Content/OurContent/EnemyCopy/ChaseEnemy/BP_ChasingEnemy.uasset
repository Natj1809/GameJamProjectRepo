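; Chasing enemy character that drives its AI through blackboard flags for arena, attack, stagger and door states.
; The player entering AttackRadius sets Attacking; the Attack event quits the game if the player is still inside, otherwise clears the flag.
; Damage briefly switches movement to Flying while staggered, with Stagger applying horizontal knockback force.
; At zero health it notifies Master and destroys itself.
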(event OnComponentBeginOverlap(AttackRadius)
  (params (OverlappedComponent :type Primitive%20Component%20Object%20Reference) (OtherActor :type Actor%20Object%20Reference) (OtherComp :type Primitive%20Component%20Object%20Reference) (OtherBodyIndex :type Integer) (bFromSweep :type Boolean) (SweepResult :type Hit%20Result%20Structure%20%28by%20ref%29))
  (if (Actor|ActorHasTag OtherActor "Player")
    (AI|Components|Blackboard|SetValueasBool (AI|GetBlackboard (AI|GetAIController self)) (Utilities|Name|MakeLiteralName "Attacking") true)))

(event Custom|Stop
  (AI|Components|Blackboard|SetValueasBool (AI|GetBlackboard (AI|GetAIController self)) (Utilities|Name|MakeLiteralName "Staggering") false)
  (Pawn|Components|CharacterMovement|SetMovementMode (Variables|Character|GetCharacterMovement) "MOVE_Walking" 0))

(event EventBeginPlay
  (|CallParentFunction)
  (AI|Components|Blackboard|SetValueasBool (AI|GetBlackboard (AI|GetAIController self)) (Utilities|Name|MakeLiteralName "InArena") false))

(event Collision|EventActorBeginOverlap
  (params (OtherActor :type Actor%20Object%20Reference))
  (|CallParentFunction OtherActor) ; This node is disabled and will not be called.\nDrag off pins to build functionality.
)

(event EventAttack
  (for _array_element (Collision|GetOverlappingActors (Variables|Default|GetAttackRadius) 0 :!class /Script/Engine.PrimitiveComponent)
    (if (Actor|ActorHasTag _array_element "Player")
      (Game|QuitGame 0 "Quit" false)))
  (AI|Components|Blackboard|SetValueasBool (AI|GetBlackboard (AI|GetAIController self)) (Utilities|Name|MakeLiteralName "Attacking") false))

(event EventDamage
  (params (Damage :type Float%20%28double-precision%29))
  (bind _output_get (Variables|Default|SetHealth (- (Variables|Default|GetHealth) Damage)))
  (if (<= _output_get 0.0)
    (Default|EnemyDeath (Variables|Default|GetMaster))
    (Actor|DestroyActor)
    (else
      (AI|Components|Blackboard|SetValueasBool (AI|GetBlackboard (AI|GetAIController self)) (Utilities|Name|MakeLiteralName "Staggering") true)
      (Pawn|Components|CharacterMovement|SetMovementMode (Variables|Character|GetCharacterMovement) "MOVE_Flying" 0)
      (Utilities|Time|SetTimerbyEvent (delegate Custom|Stop) 0.2))))

(event EventStagger
  (params (Direction :type Vector :default "0, 0, 0"))
  (Physics|AddForce (Variables|Character|GetCharacterMovement) (Math|Vector|MakeVector (.x Direction) (.y Direction) 0.0)))

(event EventTick
  (params (DeltaSeconds :type Float%20%28single-precision%29))
  (|CallParentFunction DeltaSeconds) ; This node is disabled and will not be called.\nDrag off pins to build functionality.
)

(event EventAtDoorSignal
  (params (Door :type BP%20Door%20Object%20Reference))
  (bind _self self)
  (bind _returnvalue (AI|GetAIController _self))
  (bind _returnvalue_2 (AI|GetBlackboard _returnvalue))
  (AI|Components|Blackboard|SetValueasBool _returnvalue_2 (Utilities|Name|MakeLiteralName "AtDoor") true)
  (AI|Components|Blackboard|SetValueasObject _returnvalue_2 (Utilities|Name|MakeLiteralName "Door") Door))

(fn ConstructionScript
  (|CallParentFunction))