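; BP_Door is a destructible door that alerts enemies on contact and can be broken down.
; When an actor implementing BPI_Enemy begins overlapping its Box, the door sends it AtDoorSignalMessage with a reference to itself.
; Its TakeDamage event subtracts the incoming damage from DoorHealth and destroys the actor once health reaches zero or below.
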(event OnComponentBeginOverlap(Box)
  (params (OverlappedComponent :type Primitive%20Component%20Object%20Reference) (OtherActor :type Actor%20Object%20Reference) (OtherComp :type Primitive%20Component%20Object%20Reference) (OtherBodyIndex :type Integer) (bFromSweep :type Boolean) (SweepResult :type Hit%20Result%20Structure%20%28by%20ref%29))
  (if (Utilities|DoesObjectImplementInterface OtherActor "/Game/OurContent/EnemyCopy/BPI_Enemy.BPI_Enemy_C")
    (Class|BPIEnemy|AtDoorSignal(Message) OtherActor self)))

(event Custom|TakeDamage
  (params (DAMAGE :type Float%20%28double-precision%29))
  (bind _output_get (Variables|Default|SetDoorHealth (- (Variables|Default|GetDoorHealth) DAMAGE)))
  (if (<= _output_get 0.0)
    (Actor|DestroyActor)))

(event EventBeginPlay)

(event Collision|EventActorBeginOverlap
  (params (OtherActor :type Actor%20Object%20Reference)))

(event EventTick
  (params (DeltaSeconds :type Float%20%28single-precision%29)))

(fn ConstructionScript)