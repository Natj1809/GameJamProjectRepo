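; Campfire actor with a health pool that decays each tick while lit and can be reduced by damage or topped up.
; Light intensity scales with health, clamped between minimum and maximum.
; Refills start a cooldown proportional to the amount added, and relighting restores half health.
; Extinguish and relight fire event dispatchers; damage triggers extinguishing at zero health, but decay itself never checks for it.
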(event Custom|TakeDamage
  (params (DamageTaken :type Float%20%28double-precision%29))
  ;[1 1 1] Add or remove health from fire, with a cooldown to adding to the fire
  (Utilities|GetIsLit
    (:True
      (bind _output_get (Variables|Default|SetfireHealth (CallFunction|GetHealthChange (* DamageTaken -1.0))))
      (if (<= _output_get 0.0)
        (CallFunction|FireExtinguished)
        (else
          (CallFunction|ChangeLightIntensity))))))

(event Custom|Fire%20Extinguished
  ;[1 1 1] Set state of fire + Call event dispatcher (remember to bind events to the dispatcher)
  (Variables|Default|SetbIsLit false)
  (Variables|Default|SetfireHealth 0.0)
  (CallFunction|ChangeLightIntensity)
  (Default|CallFireWentOut))

(event Custom|FireLit
  ;[1 1 1] Set state of fire + Call event dispatcher (remember to bind events to the dispatcher)
  (Utilities|GetIsLit
    (:False
      (Variables|Default|SetbIsLit true)
      (Variables|Default|SetfireHealth (/ (Variables|Default|GetmaxFireHealth) 2.0))
      (CallFunction|ChangeLightIntensity)
      (Default|CallFireRelit))))

(event Custom|FireAddedTo
  (params (AddedAmount :type Float%20%28double-precision%29))
  ;[1 1 1] Add or remove health from fire, with a cooldown to adding to the fire
  (if (Variables|Default|GetbCanBeRefilled)
    (Utilities|GetIsLit
      (:True
        (Variables|Default|SetfireHealth (CallFunction|GetHealthChange AddedAmount))
        (CallFunction|ChangeLightIntensity)
        (CallFunction|RefillCooldown (CallFunction|GetRefillCooldown AddedAmount))))))

(event Custom|FireDecay
  (params (DeltaSeconds :type Float%20%28double-precision%29))
  ;[1 1 1] Campfire health goes down over time
  (Variables|Default|SetfireHealth (- (Variables|Default|GetfireHealth) (* DeltaSeconds (Variables|Default|GetdecayAmount))))
  (CallFunction|ChangeLightIntensity))

(event Custom|ChangeLightIntensity
  ;[1 1 1] Changes how bright campfire is
  (Rendering|Components|Light|SetIntensity (Variables|Default|GetFireLight) (CallFunction|GetLightIntensity)))

(event Custom|Refill%20Cooldown
  (params (Cooldown :type Float%20%28double-precision%29))
  ;[1 1 1] Adds cooldown to refilling the fire
  (Variables|Default|SetbCanBeRefilled false)
  (Utilities|FlowControl|Delay Cooldown)
  (Variables|Default|SetbCanBeRefilled true))

(event EventBeginPlay)

(event Collision|EventActorBeginOverlap
  (params (OtherActor :type Actor%20Object%20Reference)))

(event EventTick
  (params (DeltaSeconds :type Float%20%28single-precision%29))
  ;[1 1 1] Calls fire decay while the fire is lit
  (Utilities|GetIsLit
    (:True
      (CallFunction|FireDecay DeltaSeconds))))

(fn ConstructionScript
  (Rendering|Components|Light|SetIntensity (Variables|Default|GetFireLight) (Variables|Default|GetmaxIntensity)))

(fn GetLightIntensity
  ;[1 1 1] Get new light intensity based on fire health
  (return (Math|Float|Clamp(Float) (* (Variables|Default|GetmaxIntensity) (/ (Variables|Default|GetfireHealth) (Variables|Default|GetmaxFireHealth))) (LocalVariables|GetMinIntensity) (Variables|Default|GetmaxIntensity))))

(fn GetHealthChange
  (params (Change :type Float%20%28double-precision%29))
  ;[1 1 1] gets a value for health change for the fire
  (return (Math|Float|Clamp(Float) (+ (Variables|Default|GetfireHealth) Change) 0.0 (Variables|Default|GetmaxFireHealth))))

(fn GetRefillCooldown
  (params (AmountRefilled :type Float%20%28double-precision%29))
  ;[1 1 1] Gets how long until the player can next refill this fire
  (return (* (Variables|Default|GetsecondsToRefillAll) (/ AmountRefilled (Variables|Default|GetmaxFireHealth)))))